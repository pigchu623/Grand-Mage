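; Actor Blueprint from a character VFX pack that moves a skeletal mesh along a spline path once play begins.
; The MoveCharecter timeline's Distance track is scaled by spline length to sample location and rotation on each update.
; The mesh takes the world-space location and the local-space spline rotation, with a -90 degree yaw offset applied to its relative rotation.
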(event EventBeginPlay
  (bind _spline (Variables|Default|GetSpline))
  (bind _distance (Timeline|MoveCharecter Play)
    (:Update
      (Transformation|SetWorldLocation (Variables|Default|GetSkeletalMesh) (Spline|GetLocationatDistanceAlongSpline _spline (* _distance (Spline|GetSplineLength (Variables|Default|GetSpline))) "World") false false)
      (Transformation|SetRelativeRotation (Variables|Default|GetSkeletalMesh) (Math|Rotator|MakeRotator (.roll (Spline|GetRotationatDistanceAlongSpline _spline (* _distance (Spline|GetSplineLength (Variables|Default|GetSpline))) "Local")) (.pitch (Spline|GetRotationatDistanceAlongSpline _spline (* _distance (Spline|GetSplineLength (Variables|Default|GetSpline))) "Local")) (+ (.yaw (Spline|GetRotationatDistanceAlongSpline _spline (* _distance (Spline|GetSplineLength (Variables|Default|GetSpline))) "Local")) -9e+01)) false false))))

(fn ConstructionScript)