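; BP_SplineTool is a construction-script tool from the StylizedToonWater content that lays a chosen mesh and material along a spline.
; It adds a spline mesh component per segment, with length set by XScale and actor X scale, and cross-section scale by YScale.
; Tangents are clamped to segment length to follow the curve.
; StretchMesh adds a final segment covering the leftover distance; otherwise only whole segments are placed.
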(fn ConstructionScript
  (bind _y_scale (Variables|Default|GetY%20Scale))
  (bind _spline (Variables|Default|GetSpline))
  (bind _returnvalue (Math|Conversions|ToVector(Float) _y_scale))
  (bind _returnvalue_2 (Math|Conversions|ToVector2D(Vector) _returnvalue))
  (Variables|Default|SetSpline%20Length (* (.x (Transformation|GetActorScale3D)) (* (Variables|Default|GetX%20Scale) 1e+02)))
  (if (Variables|Default|GetStretch%20Mesh?)
    (for _index (range 0 (Math|Float|Truncate (/ (Spline|GetSplineLength (Variables|Default|GetSpline)) (Variables|Default|GetSpline%20Length))))
      (Variables|Default|SetLoop%20Index _index)
      (bind _returnvalue_3 (AddComponent|AddSplineMeshComponent false))
      (Rendering|Material|SetMaterial _returnvalue_3 0 (Variables|Default|GetMaterial))
      (SplineMesh|SetStartScale _returnvalue_3 _returnvalue_2 true :!class /Script/Engine.SplineMeshComponent)
      (SplineMesh|SetEndScale _returnvalue_3 _returnvalue_2 true :!class /Script/Engine.SplineMeshComponent)
      (Components|StaticMesh|SetStaticMesh _returnvalue_3 (Variables|Default|GetMesh))
      (SplineMesh|SetForwardAxis _returnvalue_3 "X" true)
      (SplineMesh|SetStartandEnd _returnvalue_3 (Spline|GetLocationatDistanceAlongSpline _spline (* (Variables|Default|GetLoop%20Index) (Variables|Default|GetSpline%20Length)) "Local") (Math|Vector|ClampVectorSize (Spline|GetTangentatDistanceAlongSpline _spline (* (Variables|Default|GetLoop%20Index) (Variables|Default|GetSpline%20Length)) "Local") 0.0 (Variables|Default|GetSpline%20Length)) (Spline|GetLocationatDistanceAlongSpline _spline (* (+ (Variables|Default|GetLoop%20Index) 1) (Variables|Default|GetSpline%20Length)) "Local") (Math|Vector|ClampVectorSize (Spline|GetTangentatDistanceAlongSpline _spline (* (+ (Variables|Default|GetLoop%20Index) 1) (Variables|Default|GetSpline%20Length)) "Local") 0.0 (Variables|Default|GetSpline%20Length)) true :!class /Script/Engine.SplineMeshComponent))
    (else
      (bind _result (Math|Integer|DecrementInt (Math|Float|Truncate (/ (Spline|GetSplineLength (Variables|Default|GetSpline)) (Variables|Default|GetSpline%20Length))))
        (:%20%20
          (for _index_2 (range 0 _result)
            (Variables|Default|SetLoop%20Index _index_2)
            (bind _returnvalue_4 (AddComponent|AddSplineMeshComponent false))
            (Rendering|Material|SetMaterial _returnvalue_4 0 (Variables|Default|GetMaterial))
            (SplineMesh|SetStartScale _returnvalue_4 _returnvalue_2 true :!class /Script/Engine.SplineMeshComponent)
            (SplineMesh|SetEndScale _returnvalue_4 _returnvalue_2 true :!class /Script/Engine.SplineMeshComponent)
            (Components|StaticMesh|SetStaticMesh _returnvalue_4 (Variables|Default|GetMesh))
            (SplineMesh|SetForwardAxis _returnvalue_4 "X" true)
            (SplineMesh|SetStartandEnd _returnvalue_4 (Spline|GetLocationatDistanceAlongSpline _spline (* (Variables|Default|GetLoop%20Index) (Variables|Default|GetSpline%20Length)) "Local") (Math|Vector|ClampVectorSize (Spline|GetTangentatDistanceAlongSpline _spline (* (Variables|Default|GetLoop%20Index) (Variables|Default|GetSpline%20Length)) "Local") 0.0 (Variables|Default|GetSpline%20Length)) (Spline|GetLocationatDistanceAlongSpline _spline (* (+ (Variables|Default|GetLoop%20Index) 1) (Variables|Default|GetSpline%20Length)) "Local") (Math|Vector|ClampVectorSize (Spline|GetTangentatDistanceAlongSpline _spline (* (+ (Variables|Default|GetLoop%20Index) 1) (Variables|Default|GetSpline%20Length)) "Local") 0.0 (Variables|Default|GetSpline%20Length)) true :!class /Script/Engine.SplineMeshComponent)))))))