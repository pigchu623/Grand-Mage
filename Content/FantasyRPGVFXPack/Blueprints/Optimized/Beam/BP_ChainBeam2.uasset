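; Chain-beam effect actor that links nearby pawns, other than the first player's, with particle beams.
; BeginPlay spawns beam and target emitters and gathers pawns once with a sphere overlap around the actor.
; Each Tick re-reads pawn locations up to ChainTargetCount, running FirstBeam to the first, chaining BeamArray in overlap order and moving target effects onto them.
; Destroyed cleans up emitters by ChainTargetCount index.
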(event EventBeginPlay
  (bind _defaultsceneroot (Variables|Default|GetDefaultSceneRoot))
  (bind _beamsource (Variables|Default|GetBeamSource))
  (bind _returnvalue (Transformation|GetWorldLocation _defaultsceneroot))
  (for _index (range 0 (Variables|Default|GetChainTargetCount))
    (bind _returnvalue_2 (Effects|SpawnEmitteratLocation _beamsource _returnvalue))
    (Utilities|Array|Add (Variables|Default|GetBeamArray) _returnvalue_2)
    (bind _outactors (Collision|SphereOverlapActors _returnvalue 2e+03 (Utilities|Array|MakeArray "ObjectTypeQuery3") 0 (Utilities|Array|MakeArray (Game|Player|GetPlayerPawn 0))))
    (Variables|Default|SetPawnArray _outactors)
    (for _index_2 (range 0 (Variables|Default|GetChainTargetCount))
      (bind _returnvalue_3 (Effects|SpawnEmitteratLocation (Variables|Default|GetTargetEffectEmitter) "0, 0, 0" "0, 0, 0" "1.000000,1.000000,1.000000" false))
      (Utilities|Array|Add (Variables|Default|GetTargetEmitterArray) _returnvalue_3)))
  (bind _returnvalue_4 (Effects|SpawnEmitteratLocation _beamsource _returnvalue))
  (Variables|Default|SetFirstBeam _returnvalue_4))

(event Collision|EventActorBeginOverlap
  (params (OtherActor :type Actor%20Object%20Reference)))

(event EventDestroyed
  (for _index (range 0 (Variables|Default|GetChainTargetCount))
    (Components|DestroyComponent (Utilities|Array|Get(acopy) (Variables|Default|GetBeamArray) _index))
    (Components|DestroyComponent (Utilities|Array|Get(acopy) (Variables|Default|GetTargetEmitterArray) _index))
    (Components|DestroyComponent (Variables|Default|GetFirstBeam))))

(event EventTick
  (params (DeltaSeconds :type Float%20%28single-precision%29))
  (bind _hitloc (Variables|Default|GetHItLoc))
  (bind _returnvalue (Utilities|Array|LastIndex _hitloc))
  (if true
    (bind (_array_element _array_index) (Utilities|Array|ForEachLoopwithBreak (Variables|Default|GetPawnArray) :!label _label)
      (:LoopBody
        (Utilities|Array|Add (Variables|Default|GetHItLoc) (Transformation|GetActorLocation _array_element))
        (if (== _array_index (- (Variables|Default|GetChainTargetCount) 1))
          (goto _label Break)))
      (:Completed
        (bind (_array_element_2 _array_index_2) (Utilities|Array|ForEachLoopwithBreak _hitloc)
          (:LoopBody
            (if (== _array_index_2 0)
              (Class|ParticleSystemComponent|SetBeamTargetPoint (Variables|Default|GetFirstBeam) 0 _array_element_2)
              (Class|ParticleSystemComponent|SetBeamSourcePoint (Utilities|Array|Get(acopy) (Variables|Default|GetBeamArray) _array_index_2) 0 _array_element_2)
              (Class|ParticleSystemComponent|SetBeamTargetPoint (Utilities|Array|Get(acopy) (Variables|Default|GetBeamArray) _array_index_2) 0 (Utilities|Array|Get(acopy) _hitloc (+ _array_index_2 1)))
              (else
                (Class|ParticleSystemComponent|SetBeamSourcePoint (Utilities|Array|Get(acopy) (Variables|Default|GetBeamArray) _array_index_2) 0 _array_element_2)
                (if (== _returnvalue _array_index_2)
                  (Class|ParticleSystemComponent|SetBeamTargetPoint (Utilities|Array|Get(acopy) (Variables|Default|GetBeamArray) _array_index_2) 0 (Transformation|GetActorLocation (Utilities|Array|Get(acopy) (Variables|Default|GetPawnArray) _returnvalue)))
                  (else
                    (Class|ParticleSystemComponent|SetBeamTargetPoint (Utilities|Array|Get(acopy) (Variables|Default|GetBeamArray) _array_index_2) 0 (Utilities|Array|Get(acopy) _hitloc (+ _array_index_2 1)))))))
            (Transformation|SetWorldLocation (Utilities|Array|Get(acopy) (Variables|Default|GetTargetEmitterArray) _array_index_2) (Utilities|Array|Get(acopy) _hitloc _array_index_2) false false))
          (:Completed
            (Utilities|Array|Clear (Variables|Default|GetHItLoc))))))))

(fn ConstructionScript)